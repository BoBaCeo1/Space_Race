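; Player character for a side-view game: a flipbook-animated cat that runs, jumps, crouches and dies, with health and cash.
; Enhanced Input events move it along the Y axis, turn the sprite and pick flipbooks by falling and crouching state.
; CreateHUD async-loads a soft widget class, then health and cash changes are sent to the UI through messages.
; Health caps at 100, zero triggers death and destruction, and debug keys damage or print health.
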(event Custom|Death
  (Sprite|SetFlipbook (Variables|Default|GetSprite) "/Game/Assets/Character/Flipbok/FB_Cat_dead.FB_Cat_dead")
  (Utilities|FlowControl|Delay 0.8)
  (Actor|DestroyActor))

(event Input|EnhancedActionEvents|EnhancedInputActionIA_Movement
  (params (ActionValue :type Float%20%28double-precision%29) (ElapsedSeconds :type Float%20%28double-precision%29) (TriggeredSeconds :type Float%20%28double-precision%29) (InputAction :type Input%20Action%20Object%20Reference :default "/Game/Mechanics/Character/Inputs/Actions/IA_Movement.IA_Movement"))
  (bind _sprite (Variables|Default|GetSprite))
  (bind _sprite_2 (Variables|Default|GetSprite))
  (bind _sprite_3 (Variables|Default|GetSprite))
  (:Triggered
    (if (AI|Components|NavMovement|IsFalling (Variables|Character|GetCharacterMovement))
      (Sprite|SetFlipbook (Variables|Default|GetSprite) "/Game/Assets/Character/Flipbok/FB_Cat_fall.FB_Cat_fall")
      (elif (AI|Components|NavMovement|IsCrouching (Variables|Character|GetCharacterMovement))
        (Sprite|SetFlipbook _sprite_2 "/Game/Assets/Character/Flipbok/FB_Cat_ducking_move.FB_Cat_ducking_move")
        (else
          (Sprite|SetFlipbook _sprite_2 "/Game/Assets/Character/Flipbok/FB_Cat_run_.FB_Cat_run_"))))
    (if (> ActionValue 0.0)
      (Pawn|Input|AddMovementInput "0.000000,1.000000,0.000000" 1.0 false)
      (Transformation|SetWorldRotation _sprite "0.000000,90.000000,0.000000" false false)
      (else
        (Pawn|Input|AddMovementInput "0.000000,-1.000000,0.000000" 1.0 false)
        (Transformation|SetWorldRotation _sprite "0.000000,-90.000000,0.000000" false false))))
  (:Completed
    (if (AI|Components|NavMovement|IsFalling (Variables|Character|GetCharacterMovement))
      (Sprite|SetFlipbook (Variables|Default|GetSprite) "/Game/Assets/Character/Flipbok/FB_Cat_fall.FB_Cat_fall")
      (elif (AI|Components|NavMovement|IsCrouching (Variables|Character|GetCharacterMovement))
        (Sprite|SetFlipbook _sprite_3 "/Game/Assets/Character/Flipbok/FB_Cat_ducking_idle.FB_Cat_ducking_idle")
        (else
          (Sprite|SetFlipbook _sprite_3 "/Game/Assets/Character/Flipbok/FB_Cat_idle.FB_Cat_idle"))))))

(event Input|EnhancedActionEvents|EnhancedInputActionIA_Jump
  (params (ActionValue :type Boolean) (ElapsedSeconds :type Float%20%28double-precision%29) (TriggeredSeconds :type Float%20%28double-precision%29) (InputAction :type Input%20Action%20Object%20Reference :default "/Game/Mechanics/Character/Inputs/Actions/IA_Jump.IA_Jump"))
  (:Started
    (if (AI|Components|NavMovement|IsFalling (Variables|Character|GetCharacterMovement))
      (Sprite|SetFlipbook (Variables|Default|GetSprite) "/Game/Assets/Character/Flipbok/FB_Cat_fall.FB_Cat_fall")
      (else
        (Character|Jump)
        (Sprite|SetFlipbook (Variables|Default|GetSprite) "/Game/Assets/Character/Flipbok/FB_Cat_jump.FB_Cat_jump"))))
  (:Completed
    (Sprite|SetFlipbook (Variables|Default|GetSprite) "/Game/Assets/Character/Flipbok/FB_Cat_fall.FB_Cat_fall")))

(event Input|EnhancedActionEvents|EnhancedInputActionIA_Crouch
  (params (ActionValue :type Boolean) (ElapsedSeconds :type Float%20%28double-precision%29) (TriggeredSeconds :type Float%20%28double-precision%29) (InputAction :type Input%20Action%20Object%20Reference :default "/Game/Mechanics/Character/Inputs/Actions/IA_Crouch.IA_Crouch"))
  (:Triggered
    (if (AI|Components|NavMovement|IsFalling (Variables|Character|GetCharacterMovement))
      (Sprite|SetFlipbook (Variables|Default|GetSprite) "/Game/Assets/Character/Flipbok/FB_Cat_fall.FB_Cat_fall")
      (else
        (Character|Crouch)
        (Sprite|SetFlipbook (Variables|Default|GetSprite) "/Game/Assets/Character/Flipbok/FB_Cat_ducking_idle.FB_Cat_ducking_idle"))))
  (:Completed
    (if (AI|Components|NavMovement|IsFalling (Variables|Character|GetCharacterMovement))
      (Sprite|SetFlipbook (Variables|Default|GetSprite) "/Game/Assets/Character/Flipbok/FB_Cat_fall.FB_Cat_fall")
      (else
        (Character|UnCrouch)
        (Sprite|SetFlipbook (Variables|Default|GetSprite) "/Game/Assets/Character/Flipbok/FB_Cat_idle.FB_Cat_idle")))))

(event EventBeginPlay
  (Input|AddMappingContext (PlayerController|LocalPlayerSubsystems|GetEnhancedInputLocalPlayerSubsystem (Game|GetPlayerController 0)) "/Game/Mechanics/Character/Inputs/IMC_Player.IMC_Player" 0 "(bIgnoreAllPressedKeysUntilRelease=True,bForceImmediately=False,bNotifyUserSettings=False)")
  (Utilities|CreateHUD)
  (Class|BPIHealth|SendHealthtoUI(Message) (Utilities|ResolveSoftReference (Variables|Default|GetWBP%20Health)) (Variables|Default|GetHealth))
  (Class|BPICash|SendCashtoUI(Message) (Utilities|ResolveSoftReference (Variables|Default|GetWBP%20Cash)) (Variables|Default|GetCash)))

(event EventAddHealth
  (params (Health :type Float%20%28double-precision%29))
  (CallFunction|+-hp Health))

(event EventAddCash
  (params (Cash :type Integer))
  (CallFunction|+-cash Cash))

(event EventOnLanded
  (params (Hit :type Hit%20Result%20Structure%20%28by%20ref%29))
  (bind _sprite (Variables|Default|GetSprite))
  (if (Input|EnhancedActionValues|GetIA_Crouch)
    (Sprite|SetFlipbook _sprite "/Game/Assets/Character/Flipbok/FB_Cat_ducking_idle.FB_Cat_ducking_idle")
    (else
      (Sprite|SetFlipbook _sprite "/Game/Assets/Character/Flipbok/FB_Cat_idle.FB_Cat_idle"))))

(event Input|KeyboardEvents|DebugKeyQ
  (params (Key :type Key%20Structure :default "None") (ActionValue :type Input%20Action%20Value%20Structure))
  (:Pressed
    (CallFunction|+-hp -2e+01)))

(event Input|KeyboardEvents|DebugKeyT
  (params (Key :type Key%20Structure :default "None") (ActionValue :type Input%20Action%20Value%20Structure))
  (:Pressed
    (Development|PrintString (Utilities|String|ToString(Float) (Variables|Default|GetHealth)) true true "(R=0.000000,G=0.660000,B=1.000000,A=1.000000)" 5.0)))

(fn ConstructionScript)

(fn +-hp
  (params (Hp :type Float%20%28double-precision%29))
  (if (> (+ Hp (Variables|Default|GetHealth)) 1e+02)
    (LocalVariables|SetL_Health 1e+02)
    (else
      (bind _output_get (LocalVariables|SetL_Health (+ Hp (Variables|Default|GetHealth))))))
  (bind _output_get_2 (Variables|Default|SetHealth _output_get))
  (Class|BPIHealth|SendHealthtoUI(Message) (Utilities|ResolveSoftReference (Variables|Default|GetWBP_HUD)) _output_get_2)
  (if (<= _output_get_2 0.0)
    (CallFunction|Death))
  (return (Variables|Default|GetHealth)))

(fn +-cash
  (params (cash :type Integer))
  (bind _output_get (Variables|Default|SetCash (+ cash (Variables|Default|GetCash))))
  (Class|BPICash|SendCashtoUI(Message) (Utilities|ResolveSoftReference (Variables|Default|GetWBP%20Cash)) _output_get)
  (return _output_get))

(fn CheckWalletforAnoughCash
  (params (CashPurchase :type Integer))
  (if (<= CashPurchase (Variables|Default|GetCash))
    (return true)
    (else
      (return false))))